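; BP_RoadSpline is a construction-script road builder that lays spline mesh sections along its spline, with section length scaled by actor X scale.
; Each section gets a default NodeDataMap entry if missing and two spline meshes, one without collision and one with query and physics collision.
; AddRoadPiece fits meshes to the spline with tangents clamped to section length.
; Intersection nodes currently build identical pieces, as the cross-street child-actor logic is disconnected.
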(fn `AddRoadPiece`
  (params (Index :type Integer) (SplineMesh :type "SplineMeshComponent Object Reference") (CollisionType :type "ECollisionEnabled Enum" :default "NoCollision"))
  (bind _spline (`self.Spline`))
  (bind _spline_2 (`self.Spline`))
  (bind _returnvalue (* Index (`self.SectionLength`)))
  (bind _returnvalue_2 (* (+ Index 1) (`self.SectionLength`)))
  (`SplineMeshComponent.SetForwardAxis` SplineMesh "X" true)
  (`PrimitiveComponent.SetCollisionEnabled` SplineMesh CollisionType)
  (`SplineMeshComponent.SetStartAndEnd` SplineMesh (`SplineComponent.GetLocationAtDistanceAlongSpline` _spline _returnvalue "Local") (`KismetMathLibrary.ClampVectorSize` (`SplineComponent.GetTangentAtDistanceAlongSpline` _spline _returnvalue "Local") 0.0 (`self.SectionLength`)) (`SplineComponent.GetLocationAtDistanceAlongSpline` _spline_2 _returnvalue_2 "Local") (`KismetMathLibrary.ClampVectorSize` (`SplineComponent.GetTangentAtDistanceAlongSpline` _spline_2 _returnvalue_2 "Local") 0.0 (`self.SectionLength`)) true))

(fn `SetupIntersection`
  (params (CurrentIndex :type Integer) (NodeAtIndex :type "/Game/Blueprints/RoadNodeData Structure"))
  (`|ExecutionSequence`
    (:`then_0`
      (bind _returnvalue (`AddComponent|NODE_AddSplineMeshComponent-9`))
      (`self.AddRoadPiece` CurrentIndex _returnvalue))
    (:`then_1`
      (bind _returnvalue_2 (`AddComponent|NODE_AddSplineMeshComponent-10`))
      (`self.AddRoadPiece` CurrentIndex _returnvalue_2 "QueryAndPhysics"))))

(fn `UserConstructionScript`
  (locals (NodeAtIndex :type "/Game/Blueprints/RoadNodeData Structure") (CurrentIndex :type Integer))
  (bind _returnvalue_x (`KismetMathLibrary.BreakVector` (`self.GetActorScale3D`)))
  (set `self.SectionLength` (* _returnvalue_x 1197.0))
  (for _index (range (`KismetMathLibrary.FTrunc` (/ (`SplineComponent.GetSplineLength` (`self.Spline`)) (`self.SectionLength`))))
    (set `local.CurrentIndex` _index)
    (`|ExecutionSequence`
      (:`then_0`
        (if (not (`BlueprintMapLibrary.Map_Contains` (`self.NodeDataMap`) (`local.CurrentIndex`)))
          (`BlueprintMapLibrary.Map_Add` (`self.NodeDataMap`) (`local.CurrentIndex`) (make `/Game/Blueprints/RoadNodeData` false))))
      (:`then_1`
        (bind _output_get (set `local.NodeAtIndex` (`BlueprintMapLibrary.Map_Find` (`self.NodeDataMap`) (`local.CurrentIndex`))))
        (if (break `/Game/Blueprints/RoadNodeData` _output_get)
          (`self.SetupIntersection` (`local.CurrentIndex`) (`local.NodeAtIndex`))
          (else
            (`|ExecutionSequence`
              (:`then_0`
                (bind _returnvalue (`AddComponent|NODE_AddSplineMeshComponent-7`))
                (`self.AddRoadPiece` (`local.CurrentIndex`) _returnvalue))
              (:`then_1`
                (bind _returnvalue_2 (`AddComponent|NODE_AddSplineMeshComponent-8`))
                (`self.AddRoadPiece` (`local.CurrentIndex`) _returnvalue_2 "QueryAndPhysics")))))))))