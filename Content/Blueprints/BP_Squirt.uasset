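; BP_Squirt is a pooled projectile that damages actors it overlaps.
; ShootMe marks it busy, then after a short delay frees it, hides it and stops its movement for reuse instead of destroying it.
; Capsule overlaps apply damage through a DoOnce that resets after a brief cooldown.
; Logic to destroy surplus projectiles in an oversized pool is present but disconnected, so it never runs.
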(event `ShootMe`
  (params (bulletPool :type "Array of /Game/Blueprints/BP_Squirt Object Reference (by ref)"))
  (`|ExecutionSequence`
    (:`then_0`
      (set `self.IsFree` false)
      (`KismetSystemLibrary.Delay` 2.0)
      (set `self.IsFree` true)
      (`self.SetActorHiddenInGame` true)
      (`MovementComponent.StopMovementImmediately` (`self.ProjectileMovement`)))))

(event `self.Capsule.OnComponentBeginOverlap`
  (params (OverlappedComponent :type "PrimitiveComponent Object Reference") (OtherActor :type "Actor Object Reference") (OtherComp :type "PrimitiveComponent Object Reference") (OtherBodyIndex :type Integer) (bFromSweep :type Boolean) (SweepResult :type "HitResult Structure (by ref)"))
  (`/Engine/EditorBlueprintResources/StandardMacros.DoOnce` false :!label _label
    (:`Completed`
      (`GameplayStatics.ApplyDamage` OtherActor 10.0)
      (`KismetSystemLibrary.Delay` 0.2)
      (goto _label :!via `Reset`))))

(fn `UserConstructionScript`)